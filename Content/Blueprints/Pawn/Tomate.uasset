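; Tomato Blueprint that can be grabbed and dropped, with Paper2D flipbooks for idle, panic in the air and falling.
; Tick turns changes in Taken into single grab or drop events using two cross-resetting DoOnce gates.
; ToTheSky and ToTheGround timelines move the flipbook on Z while player input is disabled, returning to idle after landing.
; Overlaps on the Ombre (shadow) component set CantDrop.
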(event OnComponentBeginOverlap(Ombre)
  (params (OverlappedComponent :type Primitive%20Component%20Object%20Reference) (OtherActor :type Actor%20Object%20Reference) (OtherComp :type Primitive%20Component%20Object%20Reference) (OtherBodyIndex :type Integer) (bFromSweep :type Boolean) (SweepResult :type Hit%20Result%20Structure%20%28by%20ref%29))
  (Variables|Default|SetCan't%20drop true))

(event OnComponentEndOverlap(Ombre)
  (params (OverlappedComponent :type Primitive%20Component%20Object%20Reference) (OtherActor :type Actor%20Object%20Reference) (OtherComp :type Primitive%20Component%20Object%20Reference) (OtherBodyIndex :type Integer))
  (Variables|Default|SetCan't%20drop false))

(event Custom|Grabed
  (bind _returnvalue (Game|Player|GetPlayerPawn 0))
  (bind _returnvalue_2 (Game|GetPlayerController 0))
  (bind _tomateidle (Variables|Default|GetTomateIdle))
  (Variables|Default|SetPlace%20to%20grab (Transformation|GetWorldLocation _tomateidle))
  (Input|DisableInput _returnvalue _returnvalue_2)
  (bind _vectormoove (Timeline|ToTheSky PlayFromStart)
    (:Update
      (Transformation|SetWorldLocation _tomateidle (Math|Vector|MakeVector (.x (Variables|Default|GetPlace%20to%20grab)) (.y (Variables|Default|GetPlace%20to%20grab)) (+ (.z (Variables|Default|GetPlace%20to%20grab)) (.Z (Math|Vector|BreakVector _vectormoove)))) false false))
    (:Finished
      (Input|EnableInput _returnvalue _returnvalue_2))))

(event Custom|Droped
  (bind _returnvalue (Game|Player|GetPlayerPawn 0))
  (bind _returnvalue_2 (Game|GetPlayerController 0))
  (bind _tomateidle (Variables|Default|GetTomateIdle))
  (Variables|Default|SetPlace%20to%20drop (Transformation|GetWorldLocation _tomateidle))
  (Input|DisableInput _returnvalue _returnvalue_2)
  (bind _vectormoove (Timeline|ToTheGround PlayFromStart)
    (:Update
      (Transformation|SetWorldLocation _tomateidle (Math|Vector|MakeVector (.x (Variables|Default|GetPlace%20to%20drop)) (.y (Variables|Default|GetPlace%20to%20drop)) (+ (.z (Variables|Default|GetPlace%20to%20drop)) (.Z (Math|Vector|BreakVector _vectormoove)))) false false))
    (:Finished
      (Input|EnableInput _returnvalue _returnvalue_2)
      (Variables|Default|SetStates "NewEnumerator0")
      (CallFunction|UpdateAnimation))))

(event Custom|Update%20Animation
  (if (not (Variables|Default|GetLock%20Animation))
    (switch Utilities|FlowControl|Switch|SwitchonANmimation_State (Variables|Default|GetStates)
      (:NewEnumerator0
        (Sprite|SetFlipbook (Variables|Default|GetTomateIdle) "/Game/Ressources/Animations/TomateIdle.TomateIdle"))
      (:NewEnumerator1
        (Sprite|SetFlipbook (Variables|Default|GetTomateIdle) "/Game/Ressources/Animations/Tomate_panique.Tomate_panique"))
      (:NewEnumerator2
        (Sprite|SetFlipbook (Variables|Default|GetTomateIdle) "/Game/Ressources/Animations/Tomate_Chute.Tomate_Chute")))))

(event EventTick
  (params (DeltaSeconds :type Float%20%28single-precision%29))
  (if (Variables|Default|GetTaken)
    (Utilities|FlowControl|DoOnce false :!label _label
      (:Completed
        (Variables|Default|SetStates "NewEnumerator1")
        (CallFunction|UpdateAnimation)
        (CallFunction|Grabed)
        (goto _label_2 Reset)))
    (else
      (Utilities|FlowControl|DoOnce true :!label _label_2
        (:Completed
          (Variables|Default|SetStates "NewEnumerator2")
          (CallFunction|UpdateAnimation)
          (CallFunction|Droped)
          (goto _label Reset))))))

(fn ConstructionScript)