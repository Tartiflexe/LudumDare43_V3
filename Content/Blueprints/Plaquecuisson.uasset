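; Cooktop (plaque de cuisson) actor Blueprint with a clickable on/off button.
; A click on the off-button sprite component flips the OnOff boolean and swaps visibility between the on and off button sprites.
; The toggle only updates this state and the visuals, with no cooking or heating logic, and BeginPlay, overlap, Tick and the construction script are empty.
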(event OnClicked(PlaqueBouttonOff_Sprite)
  (params (TouchedComponent :type Primitive%20Component%20Object%20Reference) (ButtonPressed :type Key%20Structure))
  (if (Variables|Default|GetOn/Off)
    (Rendering|SetVisibility (Variables|Default|GetPlaqueBouttonOn_Sprite) false false)
    (Rendering|SetVisibility (Variables|Default|GetPlaqueBouttonOff_Sprite) true false)
    (Variables|Default|SetOn/Off false)
    (else
      (Rendering|SetVisibility (Variables|Default|GetPlaqueBouttonOn_Sprite) true false)
      (Rendering|SetVisibility (Variables|Default|GetPlaqueBouttonOff_Sprite) false false)
      (Variables|Default|SetOn/Off true))))

(event EventBeginPlay)

(event Collision|EventActorBeginOverlap
  (params (OtherActor :type Actor%20Object%20Reference)))

(event EventTick
  (params (DeltaSeconds :type Float%20%28single-precision%29)))

(fn ConstructionScript)