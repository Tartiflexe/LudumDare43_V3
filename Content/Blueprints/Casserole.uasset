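; Cooking pot actor that takes in released tomatoes, potatoes and carrots and keeps a count of each.
; Every tick it casts the first actor overlapping its capsule to each ingredient class and stores it if it is not marked Taken.
; A shared DoOnce gate waits briefly, increments the counter matching the stored item's class, then reopens the gate and destroys the item.
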(event Custom|Reset
  (bind _item_dans_la_casserole (Variables|Default|GetItem%20dans%20la%20casserole))
  (bind _returnvalue (Utilities|GetClass _item_dans_la_casserole))
  (Utilities|FlowControl|DoOnce false) ; enters at Reset
)

(event EventTick
  (params (DeltaSeconds :type Float%20%28single-precision%29))
  (bind _capsule (Variables|Default|GetCapsule))
  (bind _overlappingactors (Collision|GetOverlappingActors _capsule 0 :!class /Script/Engine.PrimitiveComponent))
  (bind _output (Utilities|Array|Get(acopy) _overlappingactors))
  (Utilities|FlowControl|Sequence
    (:then_0
      (bind _astomate (Utilities|Casting|CastToTomate _output))
      (if (not (Variables|/Game/Blueprints/Pawn/Tomate.Tomate_C|GetTaken _astomate))
        (Variables|Default|SetItem%20dans%20la%20casserole _astomate)
        (Utilities|FlowControl|DoOnce false :!label _label
          (:Completed
            (Utilities|FlowControl|Delay 0.85)
            (Utilities|FlowControl|Sequence
              (:then_0
                (if (== (Utilities|GetClass (Variables|Default|GetItem%20dans%20la%20casserole)) "/Game/Blueprints/Pawn/Tomate.Tomate_C")
                  (Variables|Default|SetTomato_count (+ (Variables|Default|GetTomato_count) 1))
                  (CallFunction|Reset :!label _label_2)
                  (Actor|DestroyActor (Variables|Default|GetItem%20dans%20la%20casserole))))
              (:then_1
                (if (== (Utilities|GetClass (Variables|Default|GetItem%20dans%20la%20casserole)) "/Game/Blueprints/Pawn/Potato.Potato_C")
                  (Variables|Default|Setpatate_count (+ (Variables|Default|Getpatate_count) 1))
                  (goto _label_2)))
              (:then_2
                (if (== (Utilities|GetClass (Variables|Default|GetItem%20dans%20la%20casserole)) "/Game/Blueprints/Pawn/Carotte.Carotte_C")
                  (Variables|Default|Setcarotte_count (+ (Variables|Default|Getcarotte_count) 1))
                  (goto _label_2))))))))
    (:then_1
      (bind _aspotato (Utilities|Casting|CastToPotato _output))
      (if (not (Variables|/Game/Blueprints/Pawn/Potato.Potato_C|GetTaken _aspotato))
        (Variables|Default|SetItem%20dans%20la%20casserole _aspotato)
        (goto _label)))
    (:then_2
      (bind _ascarotte (Utilities|Casting|CastToCarotte _output))
      (if (not (Variables|/Game/Blueprints/Pawn/Carotte.Carotte_C|GetTaken _ascarotte))
        (Variables|Default|SetItem%20dans%20la%20casserole _ascarotte)
        (goto _label)))))

(fn ConstructionScript)